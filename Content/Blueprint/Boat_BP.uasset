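; Player-controlled boat pawn that moves forward along its mesh's yaw and puts a HUD on screen at BeginPlay.
; MoveForward input feeds movement input and branches on an axis-value check.
; Each tick blends the mesh's physics velocity toward FloatingPawnMovement's horizontal velocity, keeping physics Z so vertical motion stays simulated.
; A separate function converts the player camera's yaw into positive degrees for the compass arrow.
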(event EventBeginPlay
  ;[1 1 1] Speedometer 화면에 표현
  (bind _returnvalue (UserInterface|CreateWidget "/Game/Widget/Speedometer/HUD/HUD.HUD_C"))
  (UserInterface|Viewport|AddtoViewport _returnvalue 0))

(event EventTick
  (params (DeltaSeconds :type Float%20%28single-precision%29))
  (bind _floatingpawnmovement (Variables|Default|GetFloatingPawnMovement))
  (bind _velocity (Variables|/Script/Engine.MovementComponent|GetVelocity _floatingpawnmovement))
  ;[1 1 1] 가속도 추가
  (bind _returnvalue (Physics|GetPhysicsLinearVelocity (Variables|Default|GetMeshComponent) "None"))
  (Physics|SetPhysicsLinearVelocity (Variables|Default|GetMeshComponent) (Math|Vector|Lerp(Vector) _returnvalue (Math|Vector|MakeVector (.x _velocity) (.y _velocity) (.Z (Math|Vector|BreakVector _returnvalue))) 0.9) false "None"))

(event Input|AxisEvents|InputAxisMoveForward
  (params (AxisValue :type Float%20%28single-precision%29))
  ;[1 1 1] MoveForward  (  + 회전 각도)
  (Pawn|Input|AddMovementInput (Math|Vector|GetForwardVector (Math|Rotator|MakeRotator 0.0 0.0 (.yaw (Transformation|GetWorldRotation (Variables|Default|GetMeshComponent))))) AxisValue false)
  (bind _output_get (Variables|Default|SetAxis%20Value AxisValue))
  (bind _returnvalue (Class|MyBoat|BIsOne _output_get))
  (if _returnvalue
    (Class|MyBoat|IsTrue)
    (else
      (Class|MyBoat|IsFalse))))

(fn ConstructionScript)

(fn UpdateDirectionDegree
  (bind _returnvalue (Game|Player|GetPlayerPawn 0))
  (bind _returnvalue_2 (Actor|GetComponentbyClass _returnvalue "/Script/Engine.CameraComponent"))
  (bind _returnvalue_3 (Transformation|GetWorldRotation _returnvalue_2))
  ;[1 1 1] compass의  arrow 움직이기
  (if (< (.yaw _returnvalue_3) 0.0)
    (Variables|Default|SetCurrentDirectionDegrees (+ (.yaw _returnvalue_3) 3.6e+02))
    (else
      (Variables|Default|SetCurrentDirectionDegrees (.yaw _returnvalue_3)))))